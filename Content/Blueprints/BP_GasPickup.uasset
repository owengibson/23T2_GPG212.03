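; BP_GasPickup is a gas pickup that adds time to BP_GameManager's CurrentTime when the player pawn overlaps its cube.
; The amount added, GasAddAmount, creeps upward on Tick within a clamped range.
; Once collected, it disables collision and hides, then reappears after a short delay.
; A Movement function interpolates from the stored start position toward a slight Y offset, but nothing in this Blueprint calls it.
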(event `self.ReceiveBeginPlay`
  (bind _returnvalue (`GameplayStatics.GetActorOfClass` "/Game/Blueprints/BP_GameManager.BP_GameManager_C"))
  (set `self.GameManager REF` _returnvalue)
  (set `self.StartingPos` (`self.K2_GetActorLocation`)))

(event `self.ReceiveTick`
  (params (DeltaSeconds :type "Float (single-precision)"))
  (set `self.GasAddAmount` (`KismetMathLibrary.FClamp` (+ (`self.GasAddAmount`) (* DeltaSeconds 0.01)) 2.5 3.5)))

(event `self.Cube.OnComponentBeginOverlap`
  (params (OverlappedComponent :type "PrimitiveComponent Object Reference") (OtherActor :type "Actor Object Reference") (OtherComp :type "PrimitiveComponent Object Reference") (OtherBodyIndex :type Integer) (bFromSweep :type Boolean) (SweepResult :type "HitResult Structure (by ref)"))
  (bind _gamemanager_ref (`self.GameManager REF`))
  (if (== OtherActor (`GameplayStatics.GetPlayerPawn` 0))
    (`self.SetActorEnableCollision` false)
    (`self.SetActorHiddenInGame` true)
    (set `/Game/Blueprints/BP_GameManager.CurrentTime` (+ (`/Game/Blueprints/BP_GameManager.CurrentTime` _gamemanager_ref) (`self.GasAddAmount`)) _gamemanager_ref)
    (`KismetSystemLibrary.Delay` 5.0)
    (`self.SetActorEnableCollision` true)
    (`self.SetActorHiddenInGame` false)))

(fn `Movement`
  (params (DeltaSeconds :type "Float (double-precision)"))
  (bind _startingpos (`self.StartingPos`))
  (`self.K2_SetActorLocation` (`KismetMathLibrary.VInterpTo` _startingpos (- _startingpos (0.0 -4.0 0.0)) DeltaSeconds 3.0)))

(fn `UserConstructionScript`)