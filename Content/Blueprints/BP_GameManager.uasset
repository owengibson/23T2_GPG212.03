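; BP_GameManager runs a countdown survival timer and ends the game when time runs out.
; On BeginPlay it sets game-only input, hides the cursor, resets CurrentTime to MaxTime and shows the BP_TimerBarWidget.
; Each Tick counts CurrentTime down and TimeLasted up.
; At zero, OnGameOver saves TimeLasted to BP_GameInstance and opens the DeathScreen level.
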(event `self.ReceiveBeginPlay`
  (bind _returnvalue (`GameplayStatics.GetPlayerController` 0))
  (`WidgetBlueprintLibrary.SetInputMode_GameOnly` _returnvalue)
  (set `PlayerController.bShowMouseCursor` false _returnvalue)
  (set `self.CurrentTime` (`self.MaxTime`))
  (bind _returnvalue_2 (`|CreateWidget` "/Game/Blueprints/BP_TimerBarWidget.BP_TimerBarWidget_C"))
  (`UserWidget.AddToViewport` _returnvalue_2 0))

(event `self.ReceiveTick`
  (params (DeltaSeconds :type "Float (single-precision)"))
  (`|ExecutionSequence`
    (:`then_0`
      (`self.DecreaseCurrentTime` DeltaSeconds))
    (:`then_1`
      (`self.IncreaseTimeLasted` DeltaSeconds))
    (:`then_2`
      (if (<= (`self.CurrentTime`) 0.0)
        (`self.OnGameOver`)))))

(event `OnGameOver`
  (bind _asbp_game_instance (cast `/Game/Blueprints/BP_GameInstance` (`GameplayStatics.GetGameInstance`)))
  (set `/Game/Blueprints/BP_GameInstance.TimeLasted` (`self.TimeLasted`) _asbp_game_instance)
  (`GameplayStatics.OpenLevel` "DeathScreen"))

(fn `DecreaseCurrentTime`
  (params (DeltaSeconds :type "Float (double-precision)"))
  (set `self.CurrentTime` (- (`self.CurrentTime`) DeltaSeconds))
  (return))

(fn `IncreaseTimeLasted`
  (params (DeltaSeconds :type "Float (double-precision)"))
  (set `self.TimeLasted` (+ DeltaSeconds (`self.TimeLasted`)))
  (return))

(fn `UserConstructionScript`)